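; ShieldManager is an actor that randomly colours the level's BP_ShieldBase shields and sets their starting health on BeginPlay.
; It shuffles the shields, then assigns each a student colour by index and applies the matching material to its Diamond.
; Each shield's health is that colour's DarknessShieldList value from CustomGameInstance, carrying damage from the dark world, minus that colour's recruited student count.
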(event `self.ReceiveBeginPlay`
  (bind _ascustom_game_instance (cast `/Game/MyContent/Blueprints/CustomGameInstance` (`GameplayStatics.GetGameInstance`)))
  (set `self.As Custom Game Instance` _ascustom_game_instance)
  (bind _outactors (`GameplayStatics.GetAllActorsOfClass` "/Game/MyContent/Blueprints/BP_ShieldBase.BP_ShieldBase_C"))
  (`KismetArrayLibrary.Array_Shuffle` _outactors)
  ;[1 1 1] For each shield, assign the next colour in order so they are randomized
  (for (_array_element _array_index) _outactors
    (bind _output_get (set `self.CurrentPortal` _array_element))
    (bind _output_get_2 (set `/Game/MyContent/Blueprints/BP_ShieldBase.Colour` (cast `/Game/MyContent/Blueprints/DataStructures/EN_StudentColours` (`KismetMathLibrary.Conv_IntToByte` _array_index)) _output_get))
    (set `self.NewColour` _output_get_2)
    ;[1 1 1] Set shield colour
    (`PrimitiveComponent.SetMaterial` (`/Game/MyContent/Blueprints/BP_ShieldBase.Diamond` (`self.CurrentPortal`)) 0 (select `/Game/MyContent/Blueprints/DataStructures/EN_StudentColours` (`self.NewColour`) :`NewEnumerator0` "/Game/MyContent/Materials/RedStudent.RedStudent" :`NewEnumerator1` "/Game/MyContent/Materials/BlueStudent.BlueStudent" :`NewEnumerator2` "/Game/MyContent/Materials/GreenStudent.GreenStudent" :`NewEnumerator3` "/Game/MyContent/Materials/OrangeStudent.OrangeStudent" :!type "MaterialInterface Object Reference"))
    ;[1 1 1] Set shield health to:
    ; Current health (after any damage dealt in dark world)
    ; --minus--
    ; Current number of recruited students in that colour
    (set `/Game/MyContent/Blueprints/BP_ShieldBase.CurrentHealth` (- (`BlueprintMapLibrary.Map_Find` (`/Game/MyContent/Blueprints/CustomGameInstance.DarknessShieldList` (`self.As Custom Game Instance`)) (`self.NewColour`)) (`BlueprintMapLibrary.Map_Find` (`/Game/MyContent/Blueprints/CustomGameInstance.RecruitedStudents` (`self.As Custom Game Instance`)) (`self.NewColour`))) (`self.CurrentPortal`))))

(fn `UserConstructionScript`)