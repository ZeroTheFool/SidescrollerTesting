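; Level manager that restores each student's state and colour when a level begins.
; ResetLevel reads name-keyed state and colour maps from CustomGameInstance, then applies enemy or student colours and destroys recruited students.
; Unknown students get a colour by index from the current world's list, are recorded in the game instance and start as enemies.
; Older GameMode and actor-keyed versions remain as unexecuted graphs.
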(event `self.ReceiveTick`
  (params (DeltaSeconds :type "Float (single-precision)")))

(event `Reset Level`
  (bind _as_game_instance (`self.As Game Instance`))
  (bind (_value _returnvalue) (`BlueprintMapLibrary.Map_Find` (`self.Student Management State by Name`) (`KismetSystemLibrary.GetDisplayName` (`self.CurrentStudent`))))
  ;[1 1 1] RESET: Only When the Level Resets: assign new colours from gamemode
  ;;[1 1 1] Get Student Data from GameMode
  (bind _ascustom_game_instance (cast `/Game/MyContent/Blueprints/CustomGameInstance` (`GameplayStatics.GetGameInstance`)))
  (set `self.As Game Instance` _ascustom_game_instance)
  (set `self.Student Management State by Name` (`/Game/MyContent/Blueprints/CustomGameInstance.StudentManagementStateByName` _ascustom_game_instance))
  (set `self.Student Management Colour by Name` (`/Game/MyContent/Blueprints/CustomGameInstance.StudentManagementColourByName` _ascustom_game_instance))
  ;;[1 1 1] Get List of Student Colours for *This* Level
  (set `self.StudentColourList` (select `/Game/MyContent/Blueprints/EN_WorldList` (`self.WorldNumber`) :`NewEnumerator0` (`/Game/MyContent/Blueprints/CustomGameInstance.StudentsWorld1` _as_game_instance) :`NewEnumerator1` (`/Game/MyContent/Blueprints/CustomGameInstance.StudentsWorld2` _as_game_instance) :`NewEnumerator2` (`/Game/MyContent/Blueprints/CustomGameInstance.StudentsWorld3` _as_game_instance) :`NewEnumerator3` (`/Game/MyContent/Blueprints/CustomGameInstance.StudentsWorld4` _as_game_instance)))
  ;;[1 1 1] Get all Students in this Level
  (bind _outactors (`GameplayStatics.GetAllActorsOfClass` "/Game/MyContent/Blueprints/StudentClass.StudentClass_C"))
  (bind _output_get (set `self.StudentsHere` _outactors))
  ;;[1 1 1] Loop Through Students
  (for (_array_element _array_index) _output_get
    (set `self.Counter` _array_index)
    (set `self.CurrentStudent` _array_element)
    (if _returnvalue
      ;;[1 1 1] Update Student with Existing Info
      (bind _output_get_2 (set `/Game/MyContent/Blueprints/StudentClass.CurrentState` _value (`self.CurrentStudent`)))
      (switch `/Game/MyContent/Blueprints/EN_StudentStates` _output_get_2
        (:`NewEnumerator0`
          (set `self.NewColourToUpdate` (`self.EnemyColour`))
          (`/Game/MyContent/Blueprints/StudentClass.UpdateIdentity` (`self.CurrentStudent`) (`self.NewColourToUpdate`) :!label _label))
        (:`NewEnumerator1`
          (bind _output_get_3 (set `self.NewColourToUpdate` (`BlueprintMapLibrary.Map_Find` (`self.Student Management Colour by Name`) (`KismetSystemLibrary.GetDisplayName` (`self.CurrentStudent`)))))
          (set `/Game/MyContent/Blueprints/StudentClass.CurrentColour` _output_get_3 (`self.CurrentStudent`))
          (goto _label))
        (:`NewEnumerator2`
          (`self.K2_DestroyActor` (`self.CurrentStudent`))))
      (else
        ;;[1 1 1] Add Student to Management Dictionary
        (bind _output_get_4 (set `/Game/MyContent/Blueprints/StudentClass.CurrentColour` (`|GetArrayItem` (`self.StudentColourList`) (`self.Counter`)) (`self.CurrentStudent`)))
        (`/Game/MyContent/Blueprints/CustomGameInstance.RecordNewStudent` (`self.As Game Instance`) (`self.CurrentStudent`) _output_get_4)
        (set `/Game/MyContent/Blueprints/StudentClass.CurrentState` "NewEnumerator0" (`self.CurrentStudent`))
        (`/Game/MyContent/Blueprints/StudentClass.UpdateIdentity` (`self.CurrentStudent`) (`self.EnemyColour`))))))

(event `self.ReceiveBeginPlay`
  (`self.Reset Level`))

(fn `Update Student`
  (params (Student :type "/Game/MyContent/Blueprints/StudentClass Object Reference"))
  (locals (StoredStudent :type "/Game/MyContent/Blueprints/StudentClass Object Reference"))
  (set `local.StoredStudent` Student)
  (bind _ascustom_game_instance (cast `/Game/MyContent/Blueprints/CustomGameInstance` (`GameplayStatics.GetGameInstance`)))
  (`/Game/MyContent/Blueprints/StudentClass.UpdateIdentity` (`local.StoredStudent`) (`BlueprintMapLibrary.Map_Find` (`self.Student Management Colour by Name`) (`KismetSystemLibrary.GetDisplayName` (`local.StoredStudent`)))))

(fn `UserConstructionScript`)