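; Shield actor with a spinning ring and a diamond whose material is set from its Colour on BeginPlay.
; When a SideScrollerCharacter component other than its MeleeBox overlaps the Box, the shield calls TakeDamage.
; TakeDamage passes the colour and a fixed zero health to CustomGameInstance's DarknessShieldDamage, destroying the actor if the returned health is zero.
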(event `self.ReceiveTick`
  (params (DeltaSeconds :type "Float (single-precision)"))
  (`KismetSystemLibrary.Delay` 0.1)
  (`SceneComponent.K2_AddRelativeRotation` (`self.Ring`) (struct :`Yaw` 5.0) false false))

(event `self.ReceiveBeginPlay`
  (`PrimitiveComponent.SetMaterial` (`self.Diamond`) 0 (select `/Game/MyContent/Blueprints/DataStructures/EN_StudentColours` (`self.Colour`) :`NewEnumerator0` "/Game/MyContent/Materials/RedStudent.RedStudent" :`NewEnumerator1` "/Game/MyContent/Materials/BlueStudent.BlueStudent" :`NewEnumerator2` "/Game/MyContent/Materials/GreenStudent.GreenStudent" :`NewEnumerator3` "/Game/MyContent/Materials/OrangeStudent.OrangeStudent" :!type "MaterialInterface Object Reference")))

(event `self.ReceiveActorBeginOverlap`
  (params (OtherActor :type "Actor Object Reference")))

(event `self.ReceiveActorEndOverlap`
  (params (OtherActor :type "Actor Object Reference")))

(event `self.Box.OnComponentBeginOverlap`
  (params (OverlappedComponent :type "PrimitiveComponent Object Reference") (OtherActor :type "Actor Object Reference") (OtherComp :type "PrimitiveComponent Object Reference") (OtherBodyIndex :type Integer) (bFromSweep :type Boolean) (SweepResult :type "HitResult Structure (by ref)"))
  (bind _asside_scroller_character (cast `/Game/MyContent/Blueprints/SideScrollerCharacter` OtherActor))
  (if (!= OtherComp (`/Game/MyContent/Blueprints/SideScrollerCharacter.MeleeBox` _asside_scroller_character))
    (`self.TakeDamage`)))

(fn `TakeDamage`
  (bind _ascustom_game_instance (cast `/Game/MyContent/Blueprints/CustomGameInstance` (`GameplayStatics.GetGameInstance`)))
  (bind (_dead_ _newhealth) (`/Game/MyContent/Blueprints/CustomGameInstance.DarknessShieldDamage` _ascustom_game_instance (`self.Colour`) 0))
  (if (== _newhealth 0)
    (`self.K2_DestroyActor`)))

(fn `UserConstructionScript`)