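; BP_ReturnDoor is a portal door that sends the player back to the HubWorld level through DoorInteraction.
; Overlap with the SideScrollerCharacter toggles the visibility of its Open component.
; OpenDoor toggles Closed and Open states when InteractionPending is set, updating game instance portal records and ring materials.
; EnterDoor's destination and Dark World logic is disconnected, as is the code that caches player and game instance references.
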(event `self.ReceiveBeginPlay`
  ;[1 1 1] BEGIN: set necessary variables
)

(event `self.ReceiveActorBeginOverlap`
  (params (OtherActor :type "Actor Object Reference"))
  ;[1 1 1] OVERLAP: Check that Overlapped actor is Player and Set Door name on Player so they nkow they can interact
  (cast `/Game/MyContent/Blueprints/SideScrollerCharacter` OtherActor)
  (`SceneComponent.SetVisibility` (`self.Open`) true false))

(event `self.ReceiveActorEndOverlap`
  (params (OtherActor :type "Actor Object Reference"))
  ;[1 1 1] END OVERLAP: When Player stops overlapping, set AtThisDoor to null so they know they can't interact
  (cast `/Game/MyContent/Blueprints/SideScrollerCharacter` OtherActor)
  (`SceneComponent.SetVisibility` (`self.Open`) false false))

(event `/Game/MyContent/Blueprints/Interfaces/BPI_Doors.DoorInteraction`
  (`GameplayStatics.OpenLevel` "HubWorld"))

(fn `EnterDoor`
  ;[1 1 1] BINDING: Enter Door -- if this is the door waiting for interaction (currently overlapped) and is open
)

(fn `OpenDoor`
  ;[1 1 1] BINDING: Open/Close Current Door
  (if (`self.InteractionPending`)
    (switch `/Game/MyContent/Blueprints/DataStructures/EN_DoorStates` (`self.CurrentState`)
      (:`NewEnumerator0`
        ;;[1 1 1] if CLOSED, OPEN
        (`KismetArrayLibrary.Array_AddUnique` (`/Game/MyContent/Blueprints/CustomGameInstance.CurrentlyOpenPortals` (`self.As Custom Game Instance`)) (`KismetSystemLibrary.GetDisplayName` self))
        (set `self.CurrentState` "NewEnumerator1")
        ;;[1 1 1] Closing the Door will force a reset
        (`BlueprintMapLibrary.Map_Add` (`/Game/MyContent/Blueprints/CustomGameInstance.WorldResetList` (`self.As Custom Game Instance`)) (`self.Destination`) true)
        (`self.Update Portal Rings` "/Game/MyContent/Materials/OrangeStudent.OrangeStudent"))
      (:`NewEnumerator1`
        ;;[1 1 1] if OPEN, CLOSE -- closing should trigger world refresh somehow
        (`KismetArrayLibrary.Array_RemoveItem` (`/Game/MyContent/Blueprints/CustomGameInstance.CurrentlyOpenPortals` (`self.As Custom Game Instance`)) (`KismetSystemLibrary.GetDisplayName` self))
        (set `self.CurrentState` "NewEnumerator0")
        (`self.Update Portal Rings` "/Game/MyContent/Materials/GreenStudent.GreenStudent")))))

(fn `Update Portal Rings`
  (params (NewColour :type "Material Object Reference"))
  (`PrimitiveComponent.SetMaterial` (`self.OuterRing`) 0 (`local.NewColour`))
  (`PrimitiveComponent.SetMaterial` (`self.MidRing`) 0 (`local.NewColour`))
  (`PrimitiveComponent.SetMaterial` (`self.InnerRing`) 0 (`local.NewColour`)))

(fn `UserConstructionScript`)