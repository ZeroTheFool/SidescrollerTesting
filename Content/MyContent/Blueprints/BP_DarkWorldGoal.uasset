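; BP_DarkWorldGoal is the exit trigger of a dark world level, returning the side-scroller player to the hub.
; When a SideScrollerCharacter overlaps it, it removes the current dark portal from the game instance's ThreeDarkPortals and resets CurrentRecruit.
; It then calls the game instance's DarknessDamageSystem with a fixed amount and opens the HubWorld level.
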(event `self.ReceiveActorBeginOverlap`
  (params (OtherActor :type "Actor Object Reference"))
  (bind _asside_scroller_character (cast `/Game/MyContent/Blueprints/SideScrollerCharacter` OtherActor))
  (set `self.As Side Scroller Character` _asside_scroller_character)
  (bind _ascustom_game_instance (cast `/Game/MyContent/Blueprints/CustomGameInstance` (`GameplayStatics.GetGameInstance`)))
  (bind _output_get (set `self.As Custom Game Instance` _ascustom_game_instance))
  (`KismetArrayLibrary.Array_RemoveItem` (`/Game/MyContent/Blueprints/CustomGameInstance.ThreeDarkPortals` _output_get) (`/Game/MyContent/Blueprints/CustomGameInstance.CurrentDarkPortal` _output_get))
  (set `/Game/MyContent/Blueprints/CustomGameInstance.CurrentRecruit` 0 (`self.As Custom Game Instance`))
  (`/Game/MyContent/Blueprints/CustomGameInstance.DarknessDamageSystem` (`self.As Custom Game Instance`) 10)
  (`GameplayStatics.OpenLevel` "HubWorld"))

(fn `UserConstructionScript`)