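; Backup Blueprint of a side-scroller student actor that starts as a Frozen enemy and becomes a recruitable Student when defeated.
; GetAttacked applies damage with crit doubling; at zero health it restores the colour stored by display name in the GameInstance, updating material via UpdateIdentity.
; SetRecruitVariables registers the student with the GameInstance and shows the recruit hint.
; BeginPlay and overlap events are empty, leaving contact damage, melee hits and recruit-widget logic disconnected.
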(event `self.ReceiveBeginPlay`)

(event `self.Box.OnComponentBeginOverlap`
  (params (OverlappedComponent :type "PrimitiveComponent Object Reference") (OtherActor :type "Actor Object Reference") (OtherComp :type "PrimitiveComponent Object Reference") (OtherBodyIndex :type Integer) (bFromSweep :type Boolean) (SweepResult :type "HitResult Structure (by ref)"))
  ;[1 1 1] Overlap Events
  ;;[1 1 1] Make sure overlap is only with Player's collision capsule
)

(event `self.Box.OnComponentEndOverlap`
  (params (OverlappedComponent :type "PrimitiveComponent Object Reference") (OtherActor :type "Actor Object Reference") (OtherComp :type "PrimitiveComponent Object Reference") (OtherBodyIndex :type Integer)))

(fn `GetAttacked`
  (params (Damage :type Integer) (Critical :type Boolean))
  (if (not (`self.BeingAttacked`))
    (set `self.BeingAttacked` true)
    (bind _ascustom_game_instance (cast `/Game/MyContent/Blueprints/CustomGameInstance` (`GameplayStatics.GetGameInstance`)))
    (set `self.As Game Instance` _ascustom_game_instance)
    ;[1 1 1] Can only be attacked if Enemy
    (if (`|EnumEquality` (`self.CurrentState`) "NewEnumerator0")
      (if (`local.Critical`)
        (set `self.CritMultiplier` 2)
        (else
          (set `self.CritMultiplier` 1)))
      ;[1 1 1] Take damage, check health
      (bind _output_get (set `self.EnemyCurrentHealth` (- (`self.EnemyCurrentHealth`) (* (`local.Damage`) (`self.CritMultiplier`)))))
      (if (<= _output_get 0)
        (set `self.CurrentState` "NewEnumerator1")
        ;[1 1 1] Get colour of this student, update information
        (bind _output_get_2 (set `self.CurrentColour` (`BlueprintMapLibrary.Map_Find` (`/Game/MyContent/Blueprints/CustomGameInstance.StudentManagementColourByName` (`self.As Game Instance`)) (`KismetSystemLibrary.GetDisplayName` self))))
        (`self.UpdateIdentity` _output_get_2)
        ;[1 1 1] Convert Enemy to Student
        (`/Game/MyContent/Blueprints/CustomGameInstance.EnemyToStudent` (`self.As Game Instance`) self)
        (`self.SetRecruitVariables`)
        (else
          (set `self.BeingAttacked` false))))))

(fn `UpdateIdentity`
  (params (NewColour :type "/Game/MyContent/Blueprints/DataStructures/EN_StudentColours Enum" :default "NewEnumerator0"))
  (`PrimitiveComponent.SetMaterial` (`self.StaticMesh`) 0 (select `/Game/MyContent/Blueprints/DataStructures/EN_StudentColours` NewColour :`NewEnumerator0` "/Game/MyContent/Materials/RedStudent.RedStudent" :`NewEnumerator1` "/Game/MyContent/Materials/BlueStudent.BlueStudent" :`NewEnumerator2` "/Game/MyContent/Materials/GreenStudent.GreenStudent" :`NewEnumerator3` "/Game/MyContent/Materials/OrangeStudent.OrangeStudent" :`NewEnumerator4` "/Game/MyContent/Materials/Enemy.Enemy" :!type "MaterialInterface Object Reference"))
  (set `self.Colour` (select `/Game/MyContent/Blueprints/DataStructures/EN_StudentColours` NewColour :`NewEnumerator0` (`self.Red`) :`NewEnumerator1` (`self.Blue`) :`NewEnumerator2` (`self.Green`) :`NewEnumerator3` (`self.Orange`) :`NewEnumerator4` (`self.Black`))))

(fn `UserConstructionScript`)