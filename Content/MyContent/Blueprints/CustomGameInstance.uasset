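; Game instance that holds persistent run state: health, recruited student counts by colour, and the ally team.
; On init it builds shuffled student-colour and ally draw pools, then deals students to four worlds.
; Students' colour and state are tracked by display name; recruiting the last one present redraws that world from the pool, reshuffling when empty.
; Recruited allies join the team and leave the current level, while dropped or declined ones enter a discard pool.
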(event `self.ReceiveInit`
  (bind _basestudentpool (`self.BaseStudentPool`))
  (bind _drawstudentpool (`self.DrawStudentPool`))
  (bind _drawstudentpool_2 (`self.DrawStudentPool`))
  (bind _basestudentpool_2 (`self.BaseStudentPool`))
  (bind _drawstudentpool_3 (`self.DrawStudentPool`))
  (bind _drawstudentpool_4 (`self.DrawStudentPool`))
  (set `self.CurHealth` (`self.MaxHealth`))
  (for _ (range 21)
    (`KismetArrayLibrary.Array_Add` _basestudentpool_2 "NewEnumerator0")
    (`KismetArrayLibrary.Array_Add` _basestudentpool_2 "NewEnumerator1")
    (`KismetArrayLibrary.Array_Add` _basestudentpool_2 "NewEnumerator2")
    (`KismetArrayLibrary.Array_Add` _basestudentpool_2 "NewEnumerator3"))
  (`KismetArrayLibrary.Array_Shuffle` _basestudentpool)
  (set `self.DrawStudentPool` _basestudentpool)
  (for _ (range 4)
    (`KismetArrayLibrary.Array_Add` (`self.StudentsWorld1`) (`|GetArrayItem` _drawstudentpool_4))
    (`KismetArrayLibrary.Array_Remove` _drawstudentpool_4))
  (for _ (range 4)
    (`KismetArrayLibrary.Array_Add` (`self.StudentsWorld2`) (`|GetArrayItem` _drawstudentpool))
    (`KismetArrayLibrary.Array_Remove` _drawstudentpool))
  (for _ (range 4)
    (`KismetArrayLibrary.Array_Add` (`self.StudentsWorld3`) (`|GetArrayItem` _drawstudentpool_2))
    (`KismetArrayLibrary.Array_Remove` _drawstudentpool_2))
  (for _ (range 4)
    (`KismetArrayLibrary.Array_Add` (`self.StudentsWorld4`) (`|GetArrayItem` _drawstudentpool_3))
    (`KismetArrayLibrary.Array_Remove` _drawstudentpool_3))
  (bind _output_get (set `self.DrawAllyPool` (`self.BaseAllyPool`)))
  (`KismetArrayLibrary.Array_Shuffle` _output_get))

(fn `Add New Student`
  (bind _value (`BlueprintMapLibrary.Map_Find` (`self.StudentManagementColourByName`) (`KismetSystemLibrary.GetDisplayName` (`self.StudentObjectReference`))))
  (bind _returnvalue (+ (select `/Game/MyContent/Blueprints/DataStructures/EN_StudentColours` _value :`NewEnumerator0` (`self.RedStudents`) :`NewEnumerator1` (`self.BlueStudents`) :`NewEnumerator2` (`self.GreenStudents`) :`NewEnumerator3` (`self.OrangeStudents`)) 1))
  (switch `/Game/MyContent/Blueprints/DataStructures/EN_StudentColours` _value
    (:`NewEnumerator0`
      (set `self.RedStudents` _returnvalue))
    (:`NewEnumerator1`
      (set `self.BlueStudents` _returnvalue))
    (:`NewEnumerator2`
      (set `self.GreenStudents` _returnvalue))
    (:`NewEnumerator3`
      (set `self.OrangeStudents` _returnvalue)))
  (`BlueprintMapLibrary.Map_Add` (`self.StudentManagementStateByName`) (`KismetSystemLibrary.GetDisplayName` (`self.StudentObjectReference`)) "NewEnumerator2")
  (`Actor.K2_DestroyActor` (`self.StudentObjectReference`))
  ;[1 1 1] Increment total recruited student
  (set `self.CurrentRecruit` (+ (`self.CurrentRecruit`) 1))
  (bind _outactors (`GameplayStatics.GetAllActorsOfClass` "/Game/MyContent/Blueprints/BP_StudentClass.BP_StudentClass_C"))
  (if (== (`KismetArrayLibrary.Array_Length` _outactors) 0)
    (bind _returnvalue_2 (`GameplayStatics.GetActorOfClass` "/Game/MyContent/Blueprints/StudentManager.StudentManager_C"))
    (`self.DrawNewStudents` (`/Game/MyContent/Blueprints/StudentManager.WorldNumber` _returnvalue_2))))

(fn `AddNewAlly`
  (locals (`As Character` :type "/Game/MyContent/Blueprints/SideScrollerCharacter Object Reference"))
  (bind _asside_scroller_character (cast `/Game/MyContent/Blueprints/SideScrollerCharacter` (`GameplayStatics.GetPlayerCharacter` 0)))
  (set `local.As Character` _asside_scroller_character)
  ;[1 1 1] Room for Another Ally
  (`KismetArrayLibrary.Array_AddUnique` (`self.AllyTeam`) (`/Game/MyContent/Blueprints/SideScrollerCharacter.AllyReference` (`local.As Character`)))
  (`BlueprintMapLibrary.Map_Remove` (`self.AlliesInWorld`) (`self.CurrentLevel`))
  (`Actor.K2_DestroyActor` (`self.AllyObjectReference`)))

(fn `DiscardAlly`
  (params (AllyIndex :type Integer))
  (switch `int` AllyIndex
    (:`0`
      ;[1 1 1] An existing ally was dropped from the team, add their reference ID to the discard pool based on their index in the team array
      (`KismetArrayLibrary.Array_AddUnique` (`self.DiscardAllyPool`) (`|GetArrayItem` (`self.AllyTeam`) (`local.AllyIndex`)) :!label _label))
    (:`1`
      (goto _label))
    (:`2`
      ;[1 1 1] The new ally was not chosen, add it's reference ID to the discard pool using the set ally reference
      (`KismetArrayLibrary.Array_AddUnique` (`self.DiscardAllyPool`) (`self.AllyReference`)))))

(fn `DrawNewStudents`
  (params (WorldNum :type "/Game/MyContent/Blueprints/DataStructures/EN_WorldList Enum" :default "NewEnumerator4"))
  (bind _studentcolourlist (`self.StudentColourList`))
  (`BlueprintMapLibrary.Map_Add` (`self.WorldIndexReset`) (`local.WorldNum`) true)
  (for _ (range 4)
    (if (not (!= (`KismetArrayLibrary.Array_Length` (`self.DrawStudentPool`)) 0))
      (bind _output_get (set `self.DrawStudentPool` (`self.BaseStudentPool`)))
      (`KismetArrayLibrary.Array_Shuffle` _output_get))
    (`KismetArrayLibrary.Array_Add` (`self.StudentColourList`) (`|GetArrayItem` (`self.DrawStudentPool`)))
    (`KismetArrayLibrary.Array_Remove` (`self.DrawStudentPool`)))
  (switch `/Game/MyContent/Blueprints/DataStructures/EN_WorldList` (`local.WorldNum`)
    (:`NewEnumerator0`
      (set `self.StudentsWorld1` _studentcolourlist))
    (:`NewEnumerator1`
      (set `self.StudentsWorld2` _studentcolourlist))
    (:`NewEnumerator2`
      (set `self.StudentsWorld3` _studentcolourlist))
    (:`NewEnumerator3`
      (set `self.StudentsWorld4` _studentcolourlist))))

(fn `EnemyToStudent`
  (params (StudentRef :type "/Game/MyContent/Blueprints/BP_StudentClass Object Reference"))
  (`BlueprintMapLibrary.Map_Add` (`self.StudentManagementStateByName`) (`KismetSystemLibrary.GetDisplayName` StudentRef) "NewEnumerator1"))

(fn `RecordNewStudent`
  (params (NewStudentName :type "/Game/MyContent/Blueprints/BP_StudentClass Object Reference") (Colour :type "/Game/MyContent/Blueprints/DataStructures/EN_StudentColours Enum" :default "NewEnumerator0"))
  (`BlueprintMapLibrary.Map_Add` (`self.StudentManagementColourByName`) (`KismetSystemLibrary.GetDisplayName` (`local.NewStudentName`)) Colour)
  (`BlueprintMapLibrary.Map_Add` (`self.StudentManagementStateByName`) (`KismetSystemLibrary.GetDisplayName` (`local.NewStudentName`)) "NewEnumerator0"))