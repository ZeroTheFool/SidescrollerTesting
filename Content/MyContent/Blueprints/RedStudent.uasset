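; RedStudent is a recruitable student actor that opens a recruit prompt when its Box is overlapped.
; The overlap sets AwaitingRecruit, prints debug text, removes the player's OverviewSet widget, shows BPW_RecruitStudent and pauses the game, without checking which actor overlapped.
; It then disables Box collision and restores it after a short Delay, which waits out the pause.
; End overlap clears AwaitingRecruit, and a DestroyActor node is left unconnected.
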(event `self.ReceiveBeginPlay`)

(event `self.Box.OnComponentBeginOverlap`
  (params (OverlappedComponent :type "PrimitiveComponent Object Reference") (OtherActor :type "Actor Object Reference") (OtherComp :type "PrimitiveComponent Object Reference") (OtherBodyIndex :type Integer) (bFromSweep :type Boolean) (SweepResult :type "HitResult Structure (by ref)"))
  (bind _box (`self.Box`))
  (bind _output_get (set `self.AwaitingRecruit` true))
  (`KismetSystemLibrary.PrintString` (`KismetStringLibrary.Conv_BoolToString` _output_get))
  (`KismetSystemLibrary.PrintString` (`KismetSystemLibrary.GetDisplayName` self))
  (bind _asside_scroller_character (cast `/Game/MyContent/Blueprints/SideScrollerCharacter` (`GameplayStatics.GetPlayerCharacter` 0)))
  (bind _overviewset (`/Game/MyContent/Blueprints/SideScrollerCharacter.OverviewSet` _asside_scroller_character))
  (`/Engine/EditorBlueprintResources/StandardMacros.IsValid` _overviewset
    (:`Is Valid`
      (`Widget.RemoveFromParent` _overviewset))
    (:`Is Not Valid`
      _))
  (bind _returnvalue (`|CreateWidget` "/Game/MyContent/Widgets/BPW_RecruitStudent.BPW_RecruitStudent_C"))
  (`UserWidget.AddToViewport` _returnvalue 0)
  (`GameplayStatics.SetGamePaused` true)
  (`PrimitiveComponent.SetCollisionEnabled` _box "NoCollision")
  (`KismetSystemLibrary.Delay` 1.0)
  (`PrimitiveComponent.SetCollisionEnabled` _box "QueryAndPhysics"))

(event `self.Box.OnComponentEndOverlap`
  (params (OverlappedComponent :type "PrimitiveComponent Object Reference") (OtherActor :type "Actor Object Reference") (OtherComp :type "PrimitiveComponent Object Reference") (OtherBodyIndex :type Integer))
  (set `self.AwaitingRecruit` false))

(fn `UserConstructionScript`)