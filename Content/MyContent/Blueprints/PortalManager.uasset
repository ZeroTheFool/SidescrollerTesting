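; Portal manager that assigns each door's dark, open or closed state and material from lists held in the CustomGameInstance.
; On BeginPlay it binds to the portal refresh event, and if the dark queue is empty it seeds it with shuffled door names and starts the dark cycle.
; SetPortalStatus matches doors by display name and gives non-dark doors destinations by actor array index.
; CyclePortals is an empty stub.
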(event `self.ReceiveBeginPlay`
  (bind _ascustom_game_instance (cast `/Game/MyContent/Blueprints/CustomGameInstance` (`GameplayStatics.GetGameInstance`)))
  (bind _output_get (set `self.As Custom Game Instance` _ascustom_game_instance))
  (add `/Game/MyContent/Blueprints/CustomGameInstance.RefreshPortals` _output_get (delegate `SetPortalStatus`))
  ;[1 1 1] If Dark list is empty, add all doors to it, then set portal status. if not empty, set portal status
  (if (== (`KismetArrayLibrary.Array_Length` (`/Game/MyContent/Blueprints/CustomGameInstance.DarkPortalQueue` (`self.As Custom Game Instance`))) 0)
    (bind _outactors (`GameplayStatics.GetAllActorsOfClass` "/Game/MyContent/Blueprints/BP_DoorBase.BP_DoorBase_C"))
    (set `self.AllDoors` _outactors)
    (`KismetArrayLibrary.Array_Shuffle` (`self.AllDoors`))
    (for _array_element (`self.AllDoors`)
      (`KismetArrayLibrary.Array_AddUnique` (`/Game/MyContent/Blueprints/CustomGameInstance.DarkPortalQueue` (`self.As Custom Game Instance`)) (`KismetSystemLibrary.GetDisplayName` _array_element)))
    (`/Game/MyContent/Blueprints/CustomGameInstance.DarkPortalCycle` (`self.As Custom Game Instance`))
    (else
      (`self.SetPortalStatus`))))

(event `SetPortalStatus`
  (bind _currentdoor (`self.CurrentDoor`))
  (bind _outactors (`GameplayStatics.GetAllActorsOfClass` "/Game/MyContent/Blueprints/BP_DoorBase.BP_DoorBase_C"))
  (for (_array_element _array_index) _outactors
    (set `self.CurrentDoor` _array_element)
    (set `self.DisplayName` (`KismetSystemLibrary.GetDisplayName` (`self.CurrentDoor`)))
    (if (`KismetArrayLibrary.Array_Contains` (`/Game/MyContent/Blueprints/CustomGameInstance.ThreeDarkPortals` (`self.As Custom Game Instance`)) (`self.DisplayName`))
      ;[1 1 1] Door is in Dark list, so set to Dark properties
      (set `/Game/MyContent/Blueprints/BP_DoorBase.CurrentState` "NewEnumerator2" (`self.CurrentDoor`))
      (`PrimitiveComponent.SetMaterial` (`/Game/MyContent/Blueprints/BP_DoorBase.StaticMesh` (`self.CurrentDoor`)) 0 "/Game/MyContent/Materials/DarkPortal.DarkPortal")
      (else
        ;[1 1 1] Door not in Dark list, so it keeps it's default value
        (set `/Game/MyContent/Blueprints/BP_DoorBase.Destination` (`|GetArrayItem` (`/Game/MyContent/Blueprints/CustomGameInstance.DestinationList` (`self.As Custom Game Instance`)) _array_index) (`self.CurrentDoor`))
        ;[1 1 1] Check if door is in Open list (not present in list is index -1), if not preset, door is closed -- FOR TESTING: closed doors are green, open doors are orange
        (if (== (`KismetArrayLibrary.Array_Find` (`/Game/MyContent/Blueprints/CustomGameInstance.CurrentlyOpenPortals` (`self.As Custom Game Instance`)) (`self.DisplayName`)) -1)
          (set `/Game/MyContent/Blueprints/BP_DoorBase.CurrentState` "NewEnumerator0" _currentdoor)
          (`PrimitiveComponent.SetMaterial` (`/Game/MyContent/Blueprints/BP_DoorBase.StaticMesh` (`self.CurrentDoor`)) 0 "/Game/MyContent/Materials/GreenStudent.GreenStudent")
          (else
            (set `/Game/MyContent/Blueprints/BP_DoorBase.CurrentState` "NewEnumerator1" _currentdoor)
            (`PrimitiveComponent.SetMaterial` (`/Game/MyContent/Blueprints/BP_DoorBase.StaticMesh` (`self.CurrentDoor`)) 0 "/Game/MyContent/Materials/OrangeStudent.OrangeStudent")))))))

(fn `CyclePortals`)

(fn `UserConstructionScript`)