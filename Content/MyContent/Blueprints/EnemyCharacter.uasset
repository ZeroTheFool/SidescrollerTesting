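; EnemyCharacter is an enemy Blueprint that the side-scroller player can destroy with a melee hit.
; Its HurtBox destroys the enemy instantly when overlapped by the player's MeleeBox, with no health logic.
; PlayerRadar overlaps set and clear PlayerDetected, which this graph never reads.
; The radar only casts player 0's character without checking the overlapping actor, so any overlap can toggle detection.
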(event `self.HurtBox.OnComponentBeginOverlap`
  (params (OverlappedComponent :type "PrimitiveComponent Object Reference") (OtherActor :type "Actor Object Reference") (OtherComp :type "PrimitiveComponent Object Reference") (OtherBodyIndex :type Integer) (bFromSweep :type Boolean) (SweepResult :type "HitResult Structure (by ref)"))
  (bind _asside_scroller_character (cast `/Game/MyContent/Blueprints/SideScrollerCharacter` (`GameplayStatics.GetPlayerCharacter` 0)))
  (if (== (`/Game/MyContent/Blueprints/SideScrollerCharacter.MeleeBox` _asside_scroller_character) OtherComp)
    (`self.K2_DestroyActor`)))

(event `self.PlayerRadar.OnComponentBeginOverlap`
  (params (OverlappedComponent :type "PrimitiveComponent Object Reference") (OtherActor :type "Actor Object Reference") (OtherComp :type "PrimitiveComponent Object Reference") (OtherBodyIndex :type Integer) (bFromSweep :type Boolean) (SweepResult :type "HitResult Structure (by ref)"))
  (cast `/Game/MyContent/Blueprints/SideScrollerCharacter` (`GameplayStatics.GetPlayerCharacter` 0))
  (set `self.PlayerDetected` true))

(event `self.PlayerRadar.OnComponentEndOverlap`
  (params (OverlappedComponent :type "PrimitiveComponent Object Reference") (OtherActor :type "Actor Object Reference") (OtherComp :type "PrimitiveComponent Object Reference") (OtherBodyIndex :type Integer))
  (cast `/Game/MyContent/Blueprints/SideScrollerCharacter` (`GameplayStatics.GetPlayerCharacter` 0))
  (set `self.PlayerDetected` false))

(fn `UserConstructionScript`)