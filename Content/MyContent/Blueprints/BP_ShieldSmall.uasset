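; BP_ShieldSmall is a small, destructible coloured shield actor that the side-scroller character damages with melee attacks.
; BeginPlay gives its Diamond mesh a random student-colour material, without setting the Colour variable used for damage.
; MeleeBox overlaps damage both the game instance's darkness shield for that Colour and local health by HitStrength.
; It destroys itself when either is defeated, otherwise replaying a single floating damage widget.
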(event `self.ReceiveBeginPlay`
  (`PrimitiveComponent.SetMaterial` (`self.Diamond`) 0 (select `/Game/MyContent/Blueprints/DataStructures/EN_StudentColours` (cast `/Game/MyContent/Blueprints/DataStructures/EN_StudentColours` (`KismetMathLibrary.Conv_IntToByte` (`KismetMathLibrary.RandomInteger` 4))) :`NewEnumerator0` "/Game/MyContent/Materials/RedStudent.RedStudent" :`NewEnumerator1` "/Game/MyContent/Materials/BlueStudent.BlueStudent" :`NewEnumerator2` "/Game/MyContent/Materials/GreenStudent.GreenStudent" :`NewEnumerator3` "/Game/MyContent/Materials/OrangeStudent.OrangeStudent" :!type "MaterialInterface Object Reference")))

(event `self.ReceiveActorBeginOverlap`
  (params (OtherActor :type "Actor Object Reference")))

(event `self.Box.OnComponentBeginOverlap`
  (params (OverlappedComponent :type "PrimitiveComponent Object Reference") (OtherActor :type "Actor Object Reference") (OtherComp :type "PrimitiveComponent Object Reference") (OtherBodyIndex :type Integer) (bFromSweep :type Boolean) (SweepResult :type "HitResult Structure (by ref)"))
  (bind _asside_scroller_character (cast `/Game/MyContent/Blueprints/SideScrollerCharacter` OtherActor))
  (if (== (`/Game/MyContent/Blueprints/SideScrollerCharacter.MeleeBox` _asside_scroller_character) OtherComp)
    (`self.TakeDamage`)))

(fn `TakeDamage`
  (locals (`As Game Instance` :type "/Game/MyContent/Blueprints/CustomGameInstance Object Reference"))
  (bind _damagefloater (`self.DamageFloater`))
  (bind _ascustom_game_instance (cast `/Game/MyContent/Blueprints/CustomGameInstance` (`GameplayStatics.GetGameInstance`)))
  (bind _output_get (set `local.As Game Instance` _ascustom_game_instance))
  ;[1 1 1] Apply Damage to Shield of assigned colour
  (bind _dead_ (`/Game/MyContent/Blueprints/CustomGameInstance.DarknessShieldDamage` _output_get (`self.Colour`) 0))
  ;[1 1 1] Take damage on this shield actor
  (bind _output_get_2 (set `self.LocalShieldHealth` (- (`self.LocalShieldHealth`) (`/Game/MyContent/Blueprints/CustomGameInstance.HitStrength` (`local.As Game Instance`)))))
  ;[1 1 1] If defeated, destroy
  (if (or (== _output_get_2 0) _dead_)
    (`self.K2_DestroyActor`)
    (else
      ;[1 1 1] if NOT defeated, show floating damage widget, and play animation -- i would love it if attacking again didn't reset the animation, and mulpitple numbers could be on the screen
      (`SceneComponent.SetVisibility` _damagefloater true false)
      (bind _asbpw_floating_damage (cast `/Game/MyContent/Widgets/BPW_FloatingDamage` (`WidgetComponent.GetWidget` _damagefloater)))
      (`TextBlock.SetText` (`/Game/MyContent/Widgets/BPW_FloatingDamage.DamageValueBox` _asbpw_floating_damage) (`KismetTextLibrary.Conv_IntToText` (`/Game/MyContent/Blueprints/CustomGameInstance.TotalDamageThisAttack` (`local.As Game Instance`))))
      (`UserWidget.PlayAnimation` _asbpw_floating_damage (`/Game/MyContent/Widgets/BPW_FloatingDamage.TextFloat` _asbpw_floating_damage) 0.0 1 "Forward" 1.0 false))))

(fn `UserConstructionScript`
  (`parent.UserConstructionScript`))