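; Student actor for a side-scroller that the player can recruit or, in its Enemy state, is meant to fight.
; On BeginPlay it hides its widget and restores its state from the game mode's StudentManagement map, or registers itself there.
; Box overlap in Student state shows the widget and sets the character's StudentReference, cleared on exit; Enemy only prints a placeholder.
; UpdateIdentity derives material and colour from ColourEnum; older recruit-popup logic remains disconnected.
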(event `self.ReceiveBeginPlay`
  ;[1 1 1] Set Invisible
  (`SceneComponent.SetVisibility` (`self.Widget`) false false)
  ;[1 1 1] Check if this Actor is already in Student Management
  (bind _ascustom_game_mode (cast `/Game/MyContent/Blueprints/CustomGameMode` (`GameplayStatics.GetGameMode`)))
  (bind _output_get (set `self.Game Mode` _ascustom_game_mode))
  (bind (_value _returnvalue) (`BlueprintMapLibrary.Map_Find` (`/Game/MyContent/Blueprints/CustomGameMode.StudentManagement` _output_get) self))
  (if _returnvalue
    (set `self.CurrentState` _value)
    (else
      ;[1 1 1] If not present, Add a Self reference
      (`BlueprintMapLibrary.Map_Add` (`/Game/MyContent/Blueprints/CustomGameMode.StudentManagement` (`self.Game Mode`)) self (`self.CurrentState`)))))

(event `self.Box.OnComponentBeginOverlap`
  (params (OverlappedComponent :type "PrimitiveComponent Object Reference") (OtherActor :type "Actor Object Reference") (OtherComp :type "PrimitiveComponent Object Reference") (OtherBodyIndex :type Integer) (bFromSweep :type Boolean) (SweepResult :type "HitResult Structure (by ref)"))
  ;[1 1 1] Overlap Events
  (set `self.Other Actor` OtherActor)
  ;;[1 1 1] check the State of the Actor
  (switch `/Game/MyContent/Blueprints/EN_StudentStates` (`self.CurrentState`)
    (:`NewEnumerator0`
      ;;[1 1 1] Enemy - interaction is combat, overlapped actor should be projectile or weapon
      (`KismetSystemLibrary.PrintString` "Hello"))
    (:`NewEnumerator1`
      ;;[1 1 1] Student - interact & recruit
      (bind _asside_scroller_character (cast `/Game/MyContent/Blueprints/SideScrollerCharacter` (`self.Other Actor`)))
      (set `/Game/MyContent/Blueprints/SideScrollerCharacter.StudentReference` self _asside_scroller_character)
      (`SceneComponent.SetVisibility` (`self.Widget`) true false))))

(event `self.Box.OnComponentEndOverlap`
  (params (OverlappedComponent :type "PrimitiveComponent Object Reference") (OtherActor :type "Actor Object Reference") (OtherComp :type "PrimitiveComponent Object Reference") (OtherBodyIndex :type Integer))
  ;[1 1 1] Overlap Events
  (bind _asside_scroller_character (cast `/Game/MyContent/Blueprints/SideScrollerCharacter` OtherActor))
  (set `/Game/MyContent/Blueprints/SideScrollerCharacter.StudentReference` null _asside_scroller_character)
  (`SceneComponent.SetVisibility` (`self.Widget`) false false))

(fn `UpdateIdentity`
  (`PrimitiveComponent.SetMaterial` (`self.StaticMesh`) 0 (select `/Game/MyContent/Blueprints/EN_StudentColours` (`self.ColourEnum`) :`NewEnumerator0` "/Game/MyContent/Materials/RedStudent.RedStudent" :`NewEnumerator1` "/Game/MyContent/Materials/BlueStudent.BlueStudent" :`NewEnumerator2` "/Game/MyContent/Materials/GreenStudent.GreenStudent" :`NewEnumerator3` "/Game/MyContent/Materials/OrangeStudent.OrangeStudent" :`NewEnumerator4` "/Game/MyContent/Materials/Enemy.Enemy" :!type "MaterialInterface Object Reference"))
  (set `self.Colour` (select `/Game/MyContent/Blueprints/EN_StudentColours` (`self.ColourEnum`) :`NewEnumerator0` (`self.Red`) :`NewEnumerator1` (`self.Blue`) :`NewEnumerator2` (`self.Green`) :`NewEnumerator3` (`self.Orange`) :`NewEnumerator4` (`self.Black`))))

(fn `UserConstructionScript`)