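; BP_DoorBase is a level-transition door that sends the player to another world on overlap.
; It looks up its ToWorld key in the game instance's WorldDNS map to get the level name, and resets CurrentRecruit.
; For destinations other than HubWorld, it saves the player capsule's transform as HubReturnLocation and the character's SpawnPoint before opening the level.
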(event `self.ReceiveActorBeginOverlap`
  (params (OtherActor :type "Actor Object Reference"))
  ;[1 1 1] Check that Overlapped actor is Player (will be irrelevant when door is interactable instead of overlapping)
  (bind _asside_scroller_character (cast `/Game/MyContent/Blueprints/SideScrollerCharacter` OtherActor))
  (set `self.As Side Scroller Character` _asside_scroller_character)
  (bind _ascustom_game_instance (cast `/Game/MyContent/Blueprints/CustomGameInstance` (`GameplayStatics.GetGameInstance`)))
  (bind _output_get (set `self.As Custom Game Instance` _ascustom_game_instance))
  ;[1 1 1] Reset Recruit Value
  (set `/Game/MyContent/Blueprints/CustomGameInstance.CurrentRecruit` 0 _output_get)
  (set `self.Destination` (`BlueprintMapLibrary.Map_Find` (`/Game/MyContent/Blueprints/CustomGameInstance.WorldDNS` (`self.As Custom Game Instance`)) (`self.ToWorld`)))
  ;[1 1 1] Check the Destination of the Door
  (if (not (== (`self.Destination`) "HubWorld"))
    ;[1 1 1] Destination is Other World, Save current Location
    (bind _output_get_2 (set `/Game/MyContent/Blueprints/CustomGameInstance.HubReturnLocation` (`SceneComponent.K2_GetComponentToWorld` (`Character.CapsuleComponent` (`self.As Side Scroller Character`))) (`self.As Custom Game Instance`)))
    (set `/Game/MyContent/Blueprints/SideScrollerCharacter.SpawnPoint` _output_get_2 (`self.As Side Scroller Character`)))
  ;[1 1 1] Destination is Hub, Just Open Level
  (`GameplayStatics.OpenLevel` (`self.Destination`)))

(fn `UserConstructionScript`)