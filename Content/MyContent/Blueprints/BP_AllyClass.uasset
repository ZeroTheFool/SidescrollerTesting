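; Base ally actor for the side-scroller, showing a recruit hint when the player comes near.
; Overlap with the player's capsule stores its class reference and instance on CustomGameInstance and the character.
; Leaving hides the hint but clears only StudentObjectReference, not the ally references.
; UpdateIdentity swaps material and colour by team colour; older student-recruit popup logic remains unconnected.
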(event `self.ReceiveBeginPlay`
  (set `self.EnemyCurrentHealth` (`self.EnemyMaxHealth`))
  ;[1 1 1] Hide Interaction Widget
  (`SceneComponent.SetVisibility` (`self.RecruitHint`) false false))

(event `self.Box.OnComponentBeginOverlap`
  (params (OverlappedComponent :type "PrimitiveComponent Object Reference") (OtherActor :type "Actor Object Reference") (OtherComp :type "PrimitiveComponent Object Reference") (OtherBodyIndex :type Integer) (bFromSweep :type Boolean) (SweepResult :type "HitResult Structure (by ref)"))
  ;[1 1 1] Overlap Events
  ;;[1 1 1] Make sure overlap is only with Player's collision capsule
  (bind _asside_scroller_character (cast `/Game/MyContent/Blueprints/SideScrollerCharacter` OtherActor))
  (set `self.As Side Scroller Character` _asside_scroller_character)
  (if (== (`Character.CapsuleComponent` _asside_scroller_character) OtherComp)
    (bind _ascustom_game_instance (cast `/Game/MyContent/Blueprints/CustomGameInstance` (`GameplayStatics.GetGameInstance`)))
    (set `self.As Game Instance` _ascustom_game_instance)
    (bind _output_get (set `/Game/MyContent/Blueprints/CustomGameInstance.AllyReference` (`self.AllyReference`) (`self.As Game Instance`)))
    (set `/Game/MyContent/Blueprints/SideScrollerCharacter.AllyReference` _output_get (`self.As Side Scroller Character`))
    (bind _output_get_2 (set `/Game/MyContent/Blueprints/CustomGameInstance.AllyObjectReference` self (`self.As Game Instance`)))
    (set `/Game/MyContent/Blueprints/SideScrollerCharacter.AllyObjectReference` _output_get_2 (`self.As Side Scroller Character`))
    (`SceneComponent.SetVisibility` (`self.RecruitHint`) true false)))

(event `self.Box.OnComponentEndOverlap`
  (params (OverlappedComponent :type "PrimitiveComponent Object Reference") (OtherActor :type "Actor Object Reference") (OtherComp :type "PrimitiveComponent Object Reference") (OtherBodyIndex :type Integer))
  ;[1 1 1] Overlap Events
  (bind _asside_scroller_character (cast `/Game/MyContent/Blueprints/SideScrollerCharacter` OtherActor))
  (set `/Game/MyContent/Blueprints/SideScrollerCharacter.StudentObjectReference` null _asside_scroller_character)
  (`SceneComponent.SetVisibility` (`self.RecruitHint`) false false))

(fn `UpdateIdentity`
  (params (NewColour :type "/Game/MyContent/Blueprints/EN_StudentColours Enum" :default "NewEnumerator0"))
  (`PrimitiveComponent.SetMaterial` (`self.StaticMesh`) 0 (select `/Game/MyContent/Blueprints/EN_StudentColours` NewColour :`NewEnumerator0` "/Game/MyContent/Materials/RedStudent.RedStudent" :`NewEnumerator1` "/Game/MyContent/Materials/BlueStudent.BlueStudent" :`NewEnumerator2` "/Game/MyContent/Materials/GreenStudent.GreenStudent" :`NewEnumerator3` "/Game/MyContent/Materials/OrangeStudent.OrangeStudent" :`NewEnumerator4` "/Game/MyContent/Materials/Enemy.Enemy" :!type "MaterialInterface Object Reference"))
  (set `self.Colour` (select `/Game/MyContent/Blueprints/EN_StudentColours` NewColour :`NewEnumerator0` (`self.Red`) :`NewEnumerator1` (`self.Blue`) :`NewEnumerator2` (`self.Green`) :`NewEnumerator3` (`self.Orange`) :`NewEnumerator4` (`self.Black`))))

(fn `UserConstructionScript`)