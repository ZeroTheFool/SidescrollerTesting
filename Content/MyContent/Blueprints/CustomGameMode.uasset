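; Custom game mode that runs a repeating countdown to drive the dark portal cycle.
; BeginPlay loads the countdown length, and Tick uses a Delay as a one-second gate to decrement the remaining seconds.
; When the count drops below zero, it resets and calls DarkPortalCycle on the CustomGameInstance to update the dark portals.
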(event `self.ReceiveTick`
  (params (DeltaSeconds :type "Float (single-precision)"))
  ;[1 1 1] Every second, timer ticks down 1
  (`KismetSystemLibrary.Delay` 1.0)
  (bind _output_get (set `self.Seconds` (- (`self.Seconds`) 1)))
  ;[1 1 1] Timer ends, resets, and triggers an update of the dark portals
  (if (< _output_get 0)
    (set `self.Seconds` (`self.CountdownSeconds`))
    (bind _ascustom_game_instance (cast `/Game/MyContent/Blueprints/CustomGameInstance` (`GameplayStatics.GetGameInstance`)))
    (`/Game/MyContent/Blueprints/CustomGameInstance.DarkPortalCycle` _ascustom_game_instance)))

(event `self.ReceiveBeginPlay`
  (set `self.Seconds` (`self.CountdownSeconds`)))

(fn `UserConstructionScript`)